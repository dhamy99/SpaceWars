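; BP_PowerUp is a moving pickup that grants the player a power-up on overlap.
; Each Tick, Move translates it without sweep along the forward vector captured at BeginPlay, scaled by Speed.
; Overlapping BP_Player calls GetPowerUp and fires the OnPowerUpDestroy dispatcher, which destroys the actor after a short delay.
; The "barraInferior" tag check also fires the dispatcher, but runs only after the player cast succeeds.
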(event Custom|BeDestroyed
  ;[1 1 1] Set vector direction and dispatcher destroy
  (Utilities|FlowControl|Delay 0.2)
  (Actor|DestroyActor))

(event EventBeginPlay
  ;[1 1 1] Set vector direction and dispatcher destroy
  (Variables|Default|SetMovementVector (Transformation|GetActorForwardVector))
  (EventDispatchers|BindEventtoOnPowerUpDestroy (delegate Custom|BeDestroyed)))

(event Collision|EventActorBeginOverlap
  (params (OtherActor :type Actor%20Object%20Reference))
  ;[1 1 1] Player getting a power up
  (bind _asbp_player (Utilities|Casting|CastToBP_Player OtherActor))
  (Default|GetPowerUp _asbp_player)
  (Default|CallOnPowerUpDestroy)
  (if (Utilities|Array|ContainsItem (Variables|/Script/Engine.Actor|GetTags OtherActor) "barraInferior")
    (Default|CallOnPowerUpDestroy)))

(event EventTick
  (params (DeltaSeconds :type Float%20%28single-precision%29))
  ;[1 1 1] Movement
  (CallFunction|Move DeltaSeconds))

(fn ConstructionScript)

(fn Move
  (params (DeltaTime :type Float%20%28double-precision%29))
  (Transformation|SetActorLocation (+ (Transformation|GetActorLocation) (* (* DeltaTime (Variables|Default|GetSpeed)) (Variables|Default|GetMovementVector))) false false))