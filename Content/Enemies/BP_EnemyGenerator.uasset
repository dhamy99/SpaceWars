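; Enemy generator actor that spawns enemies on a looping timer at random scene components tagged SpawnPoint.
; Each spawn picks a random type index bounded by the game mode's Level and clamped by MaxEnemies, selecting BP_EnemyBase or BP_EnemyH.
; An enemy-destroyed handler, meant to bind to each spawn, decrements SpawnTime but never restarts the running timer.
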(event Custom|Spawn
  (bind _enemyspawned (CallFunction|SpawnEnemy))
  (bind _asbp_enemy_base (Utilities|Casting|CastToBP_EnemyBase _enemyspawned))
  (EventDispatchers|BindEventtoOnEnemyDestroy _asbp_enemy_base (delegate Custom|EnemyDestroy)))

(event Custom|EnemyDestroy
  (Variables|Default|SetSpawnTime (- (Variables|Default|GetSpawnTime) 1.0)))

(event EventBeginPlay
  (Utilities|Time|SetTimerbyEvent (delegate Custom|Spawn) (Variables|Default|GetSpawnTime) true)
  (bind _asbp_game_mode (Utilities|Casting|CastToBP_GameMode (Game|GetGameMode)))
  (Variables|Default|SetGameMode _asbp_game_mode))

(event Collision|EventActorBeginOverlap
  (params (OtherActor :type Actor%20Object%20Reference)))

(event EventTick
  (params (DeltaSeconds :type Float%20%28single-precision%29)))

(fn ConstructionScript)

(fn SpawnEnemy
  (bind _returnvalue (Actor|GetComponentsbyTag "/Script/Engine.SceneComponent" "SpawnPoint"))
  (bind _class (CallFunction|GenerateEnemybyLevel (Math|Random|RandomInteger (Variables|/Game/Blueprint/BP_GameMode.BP_GameMode_C|GetLevel (Variables|Default|GetGameMode)))))
  (Game|SpawnActorfromClass _class (Transformation|GetWorldTransform (Utilities|Array|Get(acopy) _returnvalue (Math|Random|RandomInteger (Utilities|Array|Length _returnvalue)))) "Undefined" "MultiplyWithRoot" 0 0)
  (return 0))

(fn GenerateEnemybyLevel
  (params (Type :type Integer))
  (return (Utilities|Select :Index (Math|Integer|Clamp(Integer) Type 0 (- (Variables|Default|GetMaxEnemies) 1)) :Option%200 "/Game/Enemies/BP_EnemyBase.BP_EnemyBase_C" :Option%201 "/Game/Enemies/BP_EnemyH.BP_EnemyH_C" :Option%202 0)))