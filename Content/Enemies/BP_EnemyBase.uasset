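; Base enemy actor that flies straight along its initial forward vector and periodically fires ammo.
; Tick drives movement without sweep and a timer that spawns the Ammo class at FirePoint, matching the enemy's rotation.
; Overlapping a Player-tagged actor fires the OnEnemyDestroy dispatcher, which destroys the enemy after a short delay, and notifies BP_GameMode.
; A BP_Ammo cast leading into the same death logic is unconnected, so it never runs.
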(event Custom|BeDestroyed
  ;[1 1 1] Enemy life and death setup
  (Utilities|FlowControl|Delay 0.1)
  (Actor|DestroyActor))

(event EventBeginPlay
  ;[1 1 1] Enemy life and death setup
  (Variables|Default|SetMovementVector (Transformation|GetActorForwardVector))
  (EventDispatchers|BindEventtoOnEnemyDestroy (delegate Custom|BeDestroyed)))

(event Collision|EventActorBeginOverlap
  (params (OtherActor :type Actor%20Object%20Reference))
  ;[1 1 1] Enemy damaging
  (if (Utilities|Array|ContainsItem (Variables|/Script/Engine.Actor|GetTags OtherActor) "Player")
    (Default|CallOnEnemyDestroy)
    (bind _asbp_game_mode (Utilities|Casting|CastToBP_GameMode (Game|GetGameMode)))
    (Default|EnemyDestroyed _asbp_game_mode)))

(event EventTick
  (params (DeltaSeconds :type Float%20%28single-precision%29))
  ;[1 1 1] Move and shooting
  (CallFunction|Move DeltaSeconds)
  (bind _output_get (Variables|Default|SetShootCurrentTime (+ DeltaSeconds (Variables|Default|GetShootCurrentTime))))
  (if (> _output_get (Variables|Default|GetShootDelay))
    (Variables|Default|SetShootCurrentTime 0.0)
    (CallFunction|Fire)))

(fn ConstructionScript)

(fn Move
  (params (DeltaTime :type Float%20%28double-precision%29))
  (Transformation|SetActorLocation (+ (Transformation|GetActorLocation) (* (* DeltaTime (Variables|Default|GetSpeed)) (Variables|Default|GetMovementVector))) false false))

(fn Fire
  (bind _returnvalue (Game|SpawnActorfromClass (Variables|Default|GetAmmo) (Transformation|GetWorldTransform (Variables|Default|GetfirePoint)) "Undefined" "MultiplyWithRoot" 0 0))
  (Transformation|SetActorRotation _returnvalue (Transformation|GetActorRotation)))