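; BP_Ammo is a player bullet actor that explodes on contact with enemies.
; Tick moves it along its forward vector by Speed scaled by delta time, without sweeping.
; On overlap it ignores Pawns, and for other actors tagged Enemy it spawns an explosion effect and sound, then destroys itself after DestructionDelay.
; It applies no damage and has no cleanup for shots that miss.
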(event EventBeginPlay)

(event Collision|EventActorBeginOverlap
  (params (OtherActor :type Actor%20Object%20Reference))
  ;[1 1 1] Bullet destroy
  (Utilities|Casting|CastToPawn OtherActor
    (:CastFailed
      (if (Utilities|Array|ContainsItem (Variables|/Script/Engine.Actor|GetTags OtherActor) "Enemy")
        (Effects|SpawnEmitteratLocation "/Game/StarterContent/Particles/P_Explosion.P_Explosion" (Transformation|GetActorLocation))
        (Audio|PlaySound2D "/Game/StarterContent/Audio/Explosion01.Explosion01" 1.0 1.0 0.0 0 0)
        (Utilities|FlowControl|Delay (Variables|Default|GetDestructionDelay))
        (Actor|DestroyActor)))))

(event EventTick
  (params (DeltaSeconds :type Float%20%28single-precision%29))
  ;[1 1 1] Bullet movement
  (Transformation|SetActorLocation (+ (Transformation|GetActorLocation) (* (Transformation|GetActorForwardVector) (* DeltaSeconds (Variables|Default|Getspeed)))) false false))

(fn ConstructionScript)