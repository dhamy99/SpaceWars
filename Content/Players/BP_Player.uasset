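; Player character that moves and shoots via Enhanced Input and loses lives on contact with enemies.
; Firing spawns the Ammo class at the Bullet component's transform, gated by a timer cooldown.
; Overlapping non-Pawn actors tagged Enemy triggers explosion effects and damage, notifying BP_GameMode when lives hit zero.
; Tick compounds max walk speed using Speed, which AddMovementSpeed raises toward a cap.
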(event Custom|UpdateFireColdown
  ;[1 1 1] Bullet shooting
  (Variables|Default|SetCanFire true))

(event Custom|DamagePlayer
  ;[1 1 1] Damaging player
  (Variables|Default|SetLifes (- (Variables|Default|GetLifes) 1))
  (if (== (Variables|Default|GetLifes) 0)
    (bind _asbp_game_mode (Utilities|Casting|CastToBP_GameMode (Game|GetGameMode)))
    (Default|PlayerDeath _asbp_game_mode)
    (Rendering|SetActorHiddenInGame false)))

(event Input|EnhancedActionEvents|EnhancedInputActionBP_InputMovement
  (params (ActionValue :type Vector%202D%20Structure) (ElapsedSeconds :type Float%20%28double-precision%29) (TriggeredSeconds :type Float%20%28double-precision%29) (InputAction :type Input%20Action%20Object%20Reference :default "/Game/Input/BP_InputMovement.BP_InputMovement"))
  ;[1 1 1] Player movement
  (Pawn|Input|AddMovementInput (Transformation|GetActorRightVector) (.x ActionValue) false)
  (Pawn|Input|AddMovementInput (Transformation|GetActorForwardVector) (.y ActionValue) false))

(event Input|EnhancedActionEvents|EnhancedInputActionBP_InputFire
  (params (ActionValue :type Boolean) (ElapsedSeconds :type Float%20%28double-precision%29) (TriggeredSeconds :type Float%20%28double-precision%29) (InputAction :type Input%20Action%20Object%20Reference :default "/Game/Input/BP_InputFire.BP_InputFire"))
  ;[1 1 1] Bullet shooting
  (if (Variables|Default|GetCanFire)
    (CallFunction|DoFire)
    (Variables|Default|SetCanFire false)
    (Utilities|Time|SetTimerbyEvent (delegate Custom|UpdateFireColdown) (Variables|Default|GetFireColdown))))

(event EventBeginPlay
  ;[1 1 1] Assign input mapping
  (bind _asplayer_controller (Utilities|Casting|CastToPlayerController (Pawn|GetController)))
  (Utilities|IsValid (PlayerController|LocalPlayerSubsystems|GetEnhancedInputLocalPlayerSubsystem _asplayer_controller)
    (:Is%20Valid
      (Input|AddMappingContext (PlayerController|LocalPlayerSubsystems|GetEnhancedInputLocalPlayerSubsystem _asplayer_controller) "/Game/Input/BP_InputMapping.BP_InputMapping" 0 "(bIgnoreAllPressedKeysUntilRelease=True,bForceImmediately=False,bNotifyUserSettings=False)"))))

(event Collision|EventActorBeginOverlap
  (params (OtherActor :type Actor%20Object%20Reference))
  ;[1 1 1] Player death
  (Utilities|Casting|CastToPawn OtherActor
    (:CastFailed
      (if (Utilities|Array|ContainsItem (Variables|/Script/Engine.Actor|GetTags OtherActor) "Enemy")
        (Effects|SpawnEmitteratLocation "/Game/StarterContent/Particles/P_Explosion.P_Explosion" (Transformation|GetActorLocation))
        (Audio|PlaySound2D "/Game/StarterContent/Audio/Explosion02.Explosion02" 1.0 1.0 0.0 0 0)
        (CallFunction|DamagePlayer)))))

(event EventTick
  (params (DeltaSeconds :type Float%20%28single-precision%29))
  ;[1 1 1] Movement updating
  (CallFunction|UpdateMovementSpeed DeltaSeconds))

(fn ConstructionScript)

(fn DoFire
  ;[1 1 1] Spawn bullet
  (Game|SpawnActorfromClass (Variables|Default|GetAmmo) (Transformation|GetWorldTransform (Variables|Default|GetBullet)) "Undefined" "MultiplyWithRoot" 0 0))

(fn AddMovementSpeed
  (params (addSpeed :type Float%20%28double-precision%29))
  (if (< (Variables|Default|GetSpeed) 5.0)
    (Variables|Default|SetSpeed (+ addSpeed (Variables|Default|GetSpeed)))
    (else
      (Variables|Default|SetSpeed 5.0))))

(fn UpdateMovementSpeed
  (params (deltaTime :type Float%20%28double-precision%29))
  (Utilities|Casting|CastToMovementComponent (Variables|Character|GetCharacterMovement))
  (Variables|/Script/Engine.CharacterMovementComponent|SetMaxWalkSpeed (Variables|Character|GetCharacterMovement) (+ (Class|MovementComponent|GetMaxSpeed (Variables|Character|GetCharacterMovement)) (* (Class|MovementComponent|GetMaxSpeed (Variables|Character|GetCharacterMovement)) (* (Variables|Default|GetSpeed) deltaTime)))))