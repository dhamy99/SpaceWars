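; BP_Pawn is a player pawn that moves with Enhanced Input and has a placeholder fire action.
; BeginPlay adds the input mapping context to the owning player controller.
; Movement input stores a 2D value, cleared on cancel or completion, which Tick turns into unswept actor offsets along right and forward vectors, scaled by Speed and delta time.
; Fire input only prints a debug "Hello" when started or triggered.
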(event Input|EnhancedActionEvents|EnhancedInputActionBP_InputFire
  (params (ActionValue :type Boolean) (ElapsedSeconds :type Float%20%28double-precision%29) (TriggeredSeconds :type Float%20%28double-precision%29) (InputAction :type Input%20Action%20Object%20Reference :default "/Game/Input/BP_InputFire.BP_InputFire"))
  (:Triggered
    (Development|PrintText "Hello" :!label _label))
  (:Started
    (goto _label)))

(event Input|EnhancedActionEvents|EnhancedInputActionBP_InputMovement
  (params (ActionValue :type Vector%202D%20Structure) (ElapsedSeconds :type Float%20%28double-precision%29) (TriggeredSeconds :type Float%20%28double-precision%29) (InputAction :type Input%20Action%20Object%20Reference :default "/Game/Input/BP_InputMovement.BP_InputMovement"))
  (:Triggered
    (Variables|Default|SetInputValue ActionValue))
  (:Canceled
    (Variables|Default|SetInputValue "" :!label _label))
  (:Completed
    (goto _label)))

(event EventBeginPlay
  ;[1 1 1] Assign input mapping
  (bind _asplayer_controller (Utilities|Casting|CastToPlayerController (Pawn|GetController)))
  (Utilities|IsValid (PlayerController|LocalPlayerSubsystems|GetEnhancedInputLocalPlayerSubsystem _asplayer_controller)
    (:Is%20Valid
      (Input|AddMappingContext (PlayerController|LocalPlayerSubsystems|GetEnhancedInputLocalPlayerSubsystem _asplayer_controller) "/Game/Input/BP_InputMapping.BP_InputMapping" 0 "(bIgnoreAllPressedKeysUntilRelease=True,bForceImmediately=False,bNotifyUserSettings=False)"))))

(event Collision|EventActorBeginOverlap
  (params (OtherActor :type Actor%20Object%20Reference)))

(event EventTick
  (params (DeltaSeconds :type Float%20%28single-precision%29))
  (bind _speed (Variables|Default|GetSpeed))
  (bind _inputvalue (Variables|Default|GetInputValue))
  (bind _returnvalue (* DeltaSeconds _speed))
  ;[1 1 1] Update position by input
  (Transformation|SetActorLocation (+ (+ (* (Transformation|GetActorRightVector) (* _returnvalue (.x _inputvalue))) (* (* _returnvalue (.y _inputvalue)) (Transformation|GetActorForwardVector))) (Transformation|GetActorLocation)) false false))

(fn ConstructionScript)